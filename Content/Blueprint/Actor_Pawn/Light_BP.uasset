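; Player-controlled Light that is launched by click or touch and steered by added force toward sockets.
; A Stay/Fly/Arrive/Drop state drives input, per-state camera offsets, beeps and widget updates.
; A guide arrow points toward the socket nearest by Manhattan distance, its hue set by socket index.
; ArriveSocket seats the Light via timeline; DropFloor, also fired by a flight watchdog timer, counts the result and resets the Light after a delay.
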(event Custom|Input_MoveForce
  (params (Value :type Vector))
  ;[0 1 0 0.5] 入力
  (switch Utilities|FlowControl|Switch|SwitchonEnum_LightState (Variables|Default|GetLightState) ; 飛行時のみ
    (:NewEnumerator1
      (Physics|AddForce (Variables|Default|GetLight) Value "None" true) ; 加速
    )))

(event Custom|Watchdog_Stop
  ;[0 0 1 0.5] MoveForward
  ;;[0 0 1 0.5] WatchDog
  (Utilities|Time|ClearandInvalidateTimerbyHandle (stale MouseInput|EventActorOnClicked _returnvalue)))

(event Custom|Watchdog_Event
  ;[0 0 1 0.5] MoveForward
  ;;[0 0 1 0.5] WatchDog
  (CallFunction|DropFloor))

(event EventBeginPlay
  ;[1 0 0 0.5] Widgetの表示
  (bind _returnvalue (UserInterface|CreateWidget "/Game/Blueprint/MyWidget.MyWidget_C" (Game|GetPlayerController 0)))
  (bind _output_get (Variables|Default|SetWidget _returnvalue))
  (UserInterface|Viewport|AddtoViewport _output_get 0))

(event EventTick
  (params (DeltaSeconds :type Float%20%28single-precision%29))
  (bind _result_socketdistance (デフォルト|FormulaSocketDistance))
  ;[1 1 0 0.5] Tick
  (switch Utilities|FlowControl|Switch|SwitchonEnum_LightState (Variables|Default|GetLightState)
    (:NewEnumerator0
      (Utilities|GuideArrowAngle _result_socketdistance :!label _label)
      (Utilities|GuideArrowColor _result_socketdistance))
    (:NewEnumerator1
      (goto _label))
    (:NewEnumerator2
      _)
    (:NewEnumerator3
      _))
  (Utilities|CameraMove))

(event MouseInput|EventActorOnClicked
  (params (ButtonPressed :type Key%20Structure))
  ;[0 0 1 0.5] MoveForward
  (switch Utilities|FlowControl|Switch|SwitchonEnum_LightState (Variables|Default|GetLightState) ; 待機時のみ
    (:NewEnumerator0
      (Physics|AddForce (Variables|Default|GetLight) "1000.000000,1000.000000,2500.000000" "None" true) ; 加速　Forceに初期加速度を入力
      ;;[0 0 1 0.5] WatchDog
      (bind _returnvalue (Utilities|Time|SetTimerbyEvent (delegate Custom|Watchdog_Event) (Math|Float|MakeLiteralFloat 15.0)))
      (Variables|Default|SetLightState "NewEnumerator1") ; 飛行状態に
      (Utilities|Beep) ; 発射音
      (Utilities|WidgetVisable false) ; Widgetを非表示
    )))

(event EventActorOnInputTouchEnd
  (params (FingerIndex :type ETouchIndex%20Enum :default "Touch1"))
  ;[0 0 1 0.5] MoveForward
  (switch Utilities|FlowControl|Switch|SwitchonEnum_LightState (Variables|Default|GetLightState) ; 待機時のみ
    (:NewEnumerator0
      (Physics|AddForce (Variables|Default|GetLight) "1000.000000,1000.000000,2500.000000" "None" true) ; 加速　Forceに初期加速度を入力
      ;;[0 0 1 0.5] WatchDog
      (bind _returnvalue (Utilities|Time|SetTimerbyEvent (delegate Custom|Watchdog_Event) (Math|Float|MakeLiteralFloat 15.0)))
      (Variables|Default|SetLightState "NewEnumerator1") ; 飛行状態に
      (Utilities|Beep) ; 発射音
      (Utilities|WidgetVisable false) ; Widgetを非表示
    )))

(event EventDropFloor
  (bind _returnvalue (Math|Transform|MakeTransform "25.000000,25.000000, 0"))
  (bind _returnvalue_2 (Math|Vector|MakeVector 0.0 0.0 0.0))
  (bind _widget (Variables|Default|GetWidget))
  (bind _light (Variables|Default|GetLight))
  ;[0 0.5 0.5] FallTriggerに接触した時（床に落ちた時）
  ;;[0.5 1 1 0.5 12] DropFloor#1
  (switch Utilities|FlowControl|Switch|SwitchonEnum_LightState (Variables|Default|GetLightState)
    (:NewEnumerator1
      (Class|MyWidgetInterface|AddCounter(Message) _widget false)
      ;;[0.5 1 1 0.5 12] DropFloor#2
      (Variables|Default|SetLightState "NewEnumerator3") ; 落下状態に
      (Utilities|GuideArrowVisible false) ; Arrowを非表示
      (CallFunction|WatchdogStop)
      (Utilities|Beep 2))
    (:NewEnumerator2
      (Class|MyWidgetInterface|AddCounter(Message) _widget true)))
  ;;[0.5 1 1 0.5 12] DropFloor#3
  (Utilities|FlowControl|Delay 3.0) ; 接触後３秒待機
  (Utilities|PhysicsSimulate true) ; 物理シミュレーションの再開
  ;;[0.5 1 1 0.5 12] DropFloor#4
  (Transformation|SetRelativeTransform _light _returnvalue false false) ; 二回行わないと、物理がおかしくなるので注意
  (Transformation|SetRelativeTransform _light _returnvalue true true)
  (Class|PrimitiveComponent|SetAllPhysicsLinearVelocity _light _returnvalue_2 false) ; 移動ベクトルをリセット
  (Class|PrimitiveComponent|SetAllPhysicsAngularVelocityinDegrees _light _returnvalue_2 false) ; 回転ベクトルをリセット
  ;;[0.5 1 1 0.5 12] DropFloor#5
  (Variables|Default|SetLightState "NewEnumerator0") ; 待機状態に
  (Utilities|GuideArrowVisible true) ; Arrowを再表示
  (Utilities|WidgetVisable true) ; Widgetを再表示
)

(event EventArriveSocket
  (params (ThisSocketLocation :type Vector :default "0, 0, 0") (Socket_Arrive :type Socket%20BP%20Object%20Reference))
  (bind _light (Variables|Default|GetLight))
  ;[0.5 0 0] LightがSocketに到達した時
  ;;[1 0.5 0.5 0.5] ArriveSocket#1
  (CallFunction|WatchdogStop)
  (Variables|Default|SetLightState "NewEnumerator2") ; 到着状態に変更
  ;;[1 0.5 0.5 0.5] ArriveSocket#2
  (Utilities|PhysicsSimulate false) ; 物理シミュレーションの停止
  (Utilities|GuideArrowVisible false)
  (Utilities|Beep 1)
  ;;[1 0.5 0.5 0.5] ArriveSocket#3
  (bind (_direction _alpha_r _alpha_xyz) (Timeline|Timeline_WearSocket PlayFromStart)
    (:Update
      (|Lightの移動 (Variables|/Script/Engine.SceneComponent|GetRelativeLocation _light) ThisSocketLocation (Variables|/Script/Engine.SceneComponent|GetRelativeRotation _light) _alpha_r _alpha_xyz))
    (:Finished
      (Actor|DestroyActor Socket_Arrive))))

(fn ConstructionScript)

(fn FormulaSocketDistance
  (for (_array_element _array_index) (Variables|Default|GetSocketLocation)
    (|SetBy-RefVar (Utilities|Array|Get(acopy) (LocalVariables|GetTemp) _array_index) (|((ABS(X))+(ABS(Y))) (.x (- _array_element (Transformation|GetWorldLocation (Variables|Default|GetLight)))) (.y (- _array_element (Transformation|GetWorldLocation (Variables|Default|GetLight)))))))
  (return (LocalVariables|GetTemp)))

(fn TellSocketLocation
  (params (SocketLocation :type Array%20of%20Vectors))
  (Variables|Default|SetSocketLocation SocketLocation)
  (return false))