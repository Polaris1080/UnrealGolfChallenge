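; Socket actor that receives a Light_BP and spawns SocketAndLight_BP in its place when destroyed, passing on its index.
; A blinking arrow, tinted by socket index in the construction script, marks the socket.
; Successive light overlaps step a counter that sets arrow scale and sphere radius from lookup arrays.
; The last stage zeroes the arrow and messages the light with the socket's corrected location.
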(event OnComponentBeginOverlap(Sphere_Socket)
  (params (OverlappedComponent :type Primitive%20Component%20Object%20Reference) (OtherActor :type Actor%20Object%20Reference) (OtherComp :type Primitive%20Component%20Object%20Reference) (OtherBodyIndex :type Integer) (bFromSweep :type Boolean) (SweepResult :type Hit%20Result%20Structure%20%28by%20ref%29))
  (bind _counter_overlap (Variables|Default|GetCounter_Overlap))
  ;[0 1 0] Overlap-1
  (bind _aslight_bp (Utilities|Casting|CastToLight_BP OtherActor)) ; Lightであるか確認する
  (switch int _counter_overlap
    (:Default
      ;[0 1 0] Overlap-2
      (bind _result (Math|Integer|IncrementInt _counter_overlap)
        (:%20%20
          (CallFunction|ArrowSize _result)
          (CallFunction|SphereRadius _result))))
    (:3
      ;[0 1 0] Overlap-3
      (bind _result_2 (Math|Integer|IncrementInt _counter_overlap)
        (:%20%20
          (Rendering|SetVisibility (Variables|Default|GetArrow_Socket) false false)
          (CallFunction|SphereRadius _result_2))))
    (:4
      ;[0 1 0] Overlap-4
      (Variables|/Script/Engine.ArrowComponent|SetArrowSize (Variables|Default|GetArrow_Socket) 0.0) ; Arrowを隠蔽
      (Class|TellInterface|ArriveSocket(Message) _aslight_bp (+ (Transformation|GetWorldLocation (Variables|Default|GetSocket)) (Variables|Default|GetCorrect_Bottom)) self))))

(event Custom|FlickArrow
  ;[1 0 0] 初期化
  (bind _isa (Utilities|FlowControl|FlipFlop)
    (:A
      _)
    (:B
      _))
  (Rendering|SetVisibility (Variables|Default|GetArrow_Socket) _isa false))

(event Custom|Arrow_Size
  (params (Counter_Overlap :type Integer))
  ;[0 1 1 0.5] Arrowの大きさ
  (Transformation|SetWorldScale3D (Variables|Default|GetArrow_Socket) (Utilities|Array|Get(acopy) (Variables|Setting|GetSetting_Arrow_Size) Counter_Overlap)))

(event Custom|Sphere_Radius
  (params (Counter_Overlap :type Integer))
  ;[1 0 1 0.5] Sphereの大きさ
  (Components|Sphere|SetSphereRadius (Variables|Default|GetSphere_Socket) (Utilities|Array|Get(acopy) (Variables|Setting|GetSetting_Sphere_Radius) Counter_Overlap) false))

(event EventBeginPlay
  ;[1 0 0] 初期化
  (Utilities|Time|SetTimerbyEvent (delegate Custom|FlickArrow) (Variables|Arrow|GetInterval_FlickLight) true))

(event EventDestroyed
  ;[0 0 1] Socket_Lightに変化する
  (Game|SpawnActorfromClass "/Game/Blueprint/Actor_Pawn/SocketAndLight_BP.SocketAndLight_BP_C" (Transformation|GetActorTransform) "Undefined" 0 (Variables|Default|GetIndex_Socket) 0))

(event EventDropFloor
  ;[1 1 0 0.5] 床に落ちたとき
  (bind _output_get (Variables|Default|SetIndex_Socket 0))
  (CallFunction|ArrowSize _output_get)
  (CallFunction|SphereRadius _output_get))

(fn ConstructionScript
  ;[1 1 1] Arrowの色を変化
  (Components|Arrow|SetArrowColor(LinearColor) (Variables|Default|GetArrow_Socket) (Class|KismetMathLibrary|HSVtoRGB (* (Variables|Default|GetIndex_Socket) (Variables|Arrow|GetArrowHue)) 1.0 1.0 1.0)))

(fn TellSocketLocation
  (params (SocketLocation :type Array%20of%20Vectors))
  (return false))